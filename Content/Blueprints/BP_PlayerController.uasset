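; BP_PlayerController is a player controller that handles user login and text messaging through BP_GameMode.
; LoginProcess sets PlayerID to Host on the server or Guest otherwise, calls OnUserLogin, then registers the ID with the GameMode via LoginToServer.
; SendMessage forwards the text with PlayerID to the GameMode through SendMessageToServer.
; GotMessage prints incoming messages on screen only where the controller has authority.
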(event Custom|LoginProcess
  ;[0.15 0.15 0.15 0.5] 01. 플레이어 ID 설정
  (if (Networking|IsServer)
    (Variables|Default|SetPlayerID "Host")
    (else
      (Variables|Default|SetPlayerID "Guest")))
  (Default|CallOnUserLogin (Variables|Default|GetPlayerID))
  (CallFunction|LogintoServer (Variables|Default|GetPlayerID)))

(event Custom|LoginToServer
  (params (PlayerID :type String))
  ;[0.15 0.15 0.15 0.5] 02. 플레이어 서버 로그인
  (bind _asbp_game_mode (Utilities|Casting|CastToBP_GameMode (Game|GetGameMode)))
  (Class|BaseballGameMode|LoginUser _asbp_game_mode PlayerID))

(event Custom|SendMessageToServer
  (params (PlayerID :type String) (Message :type String))
  (bind _asbp_game_mode (Utilities|Casting|CastToBP_GameMode (Game|GetGameMode)))
  (Class|BaseballGameMode|ReceiveMessagefromClient _asbp_game_mode PlayerID Message))

(event Custom|GotMessage
  (params (Message :type String))
  (if (Ability|HasAuthority)
    (Development|PrintString Message true true "(R=0.000000,G=0.660000,B=1.000000,A=1.000000)" 6e+01)))

(event EventBeginPlay)

(fn ConstructionScript)

(fn SendMessage
  (params (Message :type String))
  (CallFunction|SendMessagetoServer (Variables|Default|GetPlayerID) Message))